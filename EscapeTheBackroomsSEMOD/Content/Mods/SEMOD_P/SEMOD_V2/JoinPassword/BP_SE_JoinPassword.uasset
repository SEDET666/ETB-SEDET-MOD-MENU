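; SEMOD join-password gate actor that holds one player out of the game until they type the room password in chat.
; On BeginPlay it destroys their pawn, shows a timed Chinese subtitle prompt and starts a kick timer using settings from ModActor.
; Tick scrapes chat-message widgets for that player's name.
; A correct password respawns them and removes the message, a wrong one kicks immediately, and either destroys the actor.
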(event `KickPassPlayer`
  (if (not (`self.NoKick`))
    (`AdvancedSessionsLibrary.KickPlayer` (`self.Playercontroller`) "Incorrect password. "))
  (`self.K2_DestroyActor`))

(event `self.ReceiveBeginPlay`
  (set `self.NoKick` false)
  (bind _returnvalue (`GameplayStatics.GetActorOfClass` "/Game/Mods/SEMOD_P/ModActor.ModActor_C"))
  (bind _joinpassword_stime (`/Game/Mods/SEMOD_P/savekey/semodkey.JoinPassword_Stime` (`/Game/Mods/SEMOD_P/ModActor.semodkey` _returnvalue)))
  (`KismetSystemLibrary.K2_SetTimerDelegate` (delegate `KickPassPlayer`) _joinpassword_stime)
  (`self.K2_DestroyActor` (`Controller.K2_GetPawn` (`self.Playercontroller`)))
  (`self.NSHTEXT` (`KismetStringLibrary.Concat_StrStr` "房主使用SEMOD开启了进房密码，请在" (`KismetStringLibrary.Conv_DoubleToString` _joinpassword_stime) "秒内输入正确的进房密码，否则您将被踢出游戏! ")))

(event `self.ReceiveTick`
  (params (DeltaSeconds :type "Float (single-precision)"))
  (bind _foundwidgets (`WidgetBlueprintLibrary.GetAllWidgetsOfClass` "/Game/Multiplayer/Chat/WB_ChatMessage.WB_ChatMessage_C" false))
  (for _array_element _foundwidgets
    (bind `_真发送者` (`self.提取发送者` (`KismetTextLibrary.Conv_TextToString` (`TextBlock.GetText` (`/Game/Multiplayer/Chat/WB_ChatMessage.Username_Text` _array_element)))))
    (bind _returnvalue (`GameplayStatics.GetActorOfClass` "/Game/Mods/SEMOD_P/ModActor.ModActor_C"))
    (if (`KismetStringLibrary.EqualEqual_StrStr` (`PlayerState.GetPlayerName` (`Controller.PlayerState` (`self.Playercontroller`))) `_真发送者`)
      (if (`KismetStringLibrary.EqualEqual_StrStr` (`/Game/Mods/SEMOD_P/ModActor.JoinPassword` _returnvalue) (`KismetTextLibrary.Conv_TextToString` (`TextBlock.GetText` (`/Game/Multiplayer/Chat/WB_ChatMessage.ChatMessage_Text` _array_element))))
        (if (not (`self.NoKick`))
          (`GameModeBase.RestartPlayer` (`GameplayStatics.GetGameMode`) (`self.Playercontroller`)))
        (set `self.NoKick` true)
        (`Widget.RemoveFromParent` _array_element)
        (`self.K2_DestroyActor`)
        (else
          (set `self.NoKick` false)
          (`AdvancedSessionsLibrary.KickPlayer` (`self.Playercontroller`) "Incorrect password. ")
          (`self.K2_DestroyActor`))))))

(fn `NSHTEXT`
  (params (`文本内容` :type String))
  (bind _asmp_player_controller (cast `/Game/Multiplayer/MP_PlayerController` (`self.Playercontroller`))
    (:`then`
      _)
    (:`CastFailed`
      _))
  (`/Game/Multiplayer/MP_PlayerController.HE_Subtitle` _asmp_player_controller (make `/Game/Core/Blueprints/Structures/HorrorEvent/HE_SubtitleSeq` (`|MakeArray` (make `/Game/Core/Blueprints/Structures/HorrorEvent/HE_Subtitle` (`KismetTextLibrary.Conv_StringToText` `文本内容`) null false (struct) 20.0)))))

(fn `UserConstructionScript`)

(fn `提取发送者`
  (params (`发送者` :type String))
  (returns (`真发送者` :type String))
  (return (`KismetStringLibrary.Left` `发送者` (- (`KismetStringLibrary.Len` `发送者`) 1))))