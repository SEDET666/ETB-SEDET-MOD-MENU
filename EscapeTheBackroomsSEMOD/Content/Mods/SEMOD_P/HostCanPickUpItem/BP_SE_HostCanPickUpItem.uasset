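; Mod actor that lets the local player, presumably the host, pick up dropped items with the F key.
; On BeginPlay it destroys itself if another instance already exists.
; Each tick it line-traces from player 0's camera through screen center, matching hits by "BP_DroppedItem_" class-name prefix within a set distance.
; Matching items receive focus, F passes them to the character's InvAdd, and focus ends on pickup or look-away.
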(event `self.ReceiveBeginPlay`
  (bind _outactors (`GameplayStatics.GetAllActorsOfClass` "BP_SE_HostCanPickUpItem_C"))
  (if (> (`KismetArrayLibrary.Array_Length` _outactors) 1)
    (`self.K2_DestroyActor`))
  (set `self.REA` false))

(event `self.ReceiveTick`
  (params (DeltaSeconds :type "Float (single-precision)"))
  (bind (_actor `_距离`) (`self.射线检测` 0))
  (if (and (`KismetStringLibrary.EqualEqual_StrStr` (`KismetStringLibrary.Left` (`KismetSystemLibrary.GetClassDisplayName` (`GameplayStatics.GetObjectClass` _actor)) 15) "BP_DroppedItem_") (<= `_距离` (`self.检测距离`)))
    (bind _asbp_dropped_item (cast `/Game/NewInventorySystem/DroppedItems/BP_DroppedItem` _actor)
      (:`then`
        _)
      (:`CastFailed`
        _))
    (bind _output_get (set `self.SYGACTOR` _asbp_dropped_item))
    (`/Game/NewInventorySystem/DroppedItems/BP_DroppedItem.OnBeginFocus` _output_get)
    (set `self.REA` true)
    (if (`PlayerController.WasInputKeyJustPressed` (`GameplayStatics.GetPlayerController` 0) "F")
      (bind _asbpcharacter_demo (cast `/Game/Game/BPCharacter_Demo` (`GameplayStatics.GetPlayerPawn` 0))
        (:`then`
          _)
        (:`CastFailed`
          _))
      (`/Game/Game/BPCharacter_Demo.InvAdd` _asbpcharacter_demo _asbp_dropped_item)
      (`/Game/NewInventorySystem/DroppedItems/BP_DroppedItem.OnEndFocus` _output_get))
    (elif (`self.REA`)
      (`/Game/NewInventorySystem/DroppedItems/BP_DroppedItem.OnEndFocus` (`self.SYGACTOR`))
      (set `self.REA` false))))

(fn `UserConstructionScript`)

(fn `射线检测`
  (params (`玩家ID` :type Integer))
  (returns (Actor :type "Actor Object Reference") (`距离` :type "Float (double-precision)"))
  (bind (_returnvalue_x _returnvalue_y) (`KismetMathLibrary.BreakVector2D` (* (`WidgetLayoutLibrary.GetViewportSize`) 0.5)))
  (bind _returnvalue (`PlayerCameraManager.GetCameraLocation` (`GameplayStatics.GetPlayerCameraManager` `玩家ID`)))
  (bind _outhit (`KismetSystemLibrary.LineTraceSingle` _returnvalue (+ _returnvalue (* (`.WorldDirection` (`PlayerController.DeprojectScreenPositionToWorld` (`GameplayStatics.GetPlayerController` `玩家ID`) _returnvalue_x _returnvalue_y)) 10000.0)) "TraceTypeQuery1"))
  (bind (_bblockinghit _binitialoverlap _time _distance _location _impactpoint _normal _impactnormal _physmat _hitactor) (`GameplayStatics.BreakHitResult` _outhit))
  (return _hitactor _distance))