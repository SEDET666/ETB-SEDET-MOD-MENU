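; BP_PostSPESP is an actor from the SEMOD_P mod that applies a player ESP material as a screen-wide post-process effect.
; On BeginPlay it makes its PostProcess component unbound, creates a dynamic instance of PlayerESP_Inst and registers it as a weighted blendable.
; It then sets the material's "scope" scalar parameter to zero; overlap, tick and construction logic are empty.
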(event `self.ReceiveBeginPlay`
  (bind _postprocess (`self.PostProcess`))
  (set `PostProcessComponent.bUnbound` true (`self.PostProcess`))
  (bind _returnvalue (`KismetMaterialLibrary.CreateDynamicMaterialInstance` "/Game/Mods/SEMOD_P/ESP/PlayerESP_Inst.PlayerESP_Inst"))
  (bind _output_get (set `self.Matinstance` _returnvalue))
  (set `PostProcessComponent.Settings` (make `PostProcessSettings` :`WeightedBlendables` (make `WeightedBlendables` (`|MakeArray` (make `WeightedBlendable` -1.0 _output_get)))) _postprocess)
  (`PostProcessComponent.AddOrUpdateBlendable` _postprocess _output_get 1.0)
  (`MaterialInstanceDynamic.SetScalarParameterValue` (`self.Matinstance`) "scope" 0.0))

(event `self.ReceiveActorBeginOverlap`
  (params (OtherActor :type "Actor Object Reference")))

(event `self.ReceiveTick`
  (params (DeltaSeconds :type "Float (single-precision)")))

(fn `UserConstructionScript`)