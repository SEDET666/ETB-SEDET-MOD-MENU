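; BP_FreeocmSE is a mod pawn that mirrors the position and rotation of a referenced Bpcharacterdemo actor.
; Every Tick it copies that actor's location and rotation, teleporting without sweep.
; Movement, look and EnableInput nodes remain in the graph but are disconnected, so its input events and BeginPlay do nothing.
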(event `self.ReceiveBeginPlay`)

(event `InputAxis|LookUp`
  (params (AxisValue :type "Float (single-precision)")))

(event `self.ReceiveTick`
  (params (DeltaSeconds :type "Float (single-precision)"))
  (bind _bpcharacterdemo (`self.bpcharacterdemo`))
  (`self.K2_SetActorLocation` (`self.K2_GetActorLocation` _bpcharacterdemo) false true)
  (`self.K2_SetActorRotation` (`self.K2_GetActorRotation` _bpcharacterdemo) true))

(event `InputAxis|LookRight`
  (params (AxisValue :type "Float (single-precision)")))

(event `InputAxis|MoveForward`
  (params (AxisValue :type "Float (single-precision)")))

(event `InputAxis|MoveRight`
  (params (AxisValue :type "Float (single-precision)")))

(fn `UserConstructionScript`)